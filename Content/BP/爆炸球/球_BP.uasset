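; Exploding ball actor that assembles a rotating shell of BP_ballZs pieces, then bursts apart.
; After a startup delay it spawns the pieces at randomized transforms around the outer sphere, attaches them, spins that sphere and ramps another timeline's play rate.
; A timed boom disables collision, detaches the pieces, calls FlyZ on each with the arrow's location, fires the explosion particle and clears instances.
; The construction script's random instanced-mesh fill is disconnected.
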(event `self.ReceiveBeginPlay`
  (bind (_origin _boxextent _sphereradius) (`KismetSystemLibrary.GetComponentBounds` (`self.Sphere外圈`)))
  (`KismetSystemLibrary.Delay` (`self.Duration`))
  (`|ExecutionSequence`
    (:`then_0`
      (for _ (range 101)
        (bind _returnvalue (`|SpawnActorFromClass` "/Game/BP/爆炸球/BP_ballZs.BP_ballZs_C" (`KismetMathLibrary.MakeTransform` (+ _origin (`KismetMathLibrary.GreaterGreater_VectorRotator` (* (`SceneComponent.GetForwardVector` (`self.Sphere外圈`)) (`KismetMathLibrary.Conv_IntToDouble` (`KismetMathLibrary.RandomIntegerInRange` (`KismetMathLibrary.FTrunc` (- _sphereradius 300.0)) (`KismetMathLibrary.FTrunc` _sphereradius)))) (`KismetMathLibrary.MakeRotator` (`KismetMathLibrary.RandomFloatInRange` -180.0 180.0) (`KismetMathLibrary.RandomFloatInRange` -180.0 180.0) (`KismetMathLibrary.RandomFloatInRange` -180.0 180.0)))) (`KismetMathLibrary.MakeRotator` (`KismetMathLibrary.RandomFloatInRange` -180.0 180.0) (`KismetMathLibrary.RandomFloatInRange` -180.0 180.0) (`KismetMathLibrary.RandomFloatInRange` -180.0 180.0))) "Undefined" "OverrideRootScale" null null))
        (`self.K2_AttachToComponent` _returnvalue (`self.Sphere外圈`) "None" "KeepWorld" "KeepWorld" "KeepWorld" true)
        (`KismetArrayLibrary.Array_Add` (`self.All`) _returnvalue)))
    (:`then_1`
      (`MovementComponent.SetUpdatedComponent` (`self.RotatingMovement`) (`self.Sphere外圈`)))
    (:`then_2`
      (bind (_direction `_新建轨道_0`) (`Timeline|时间轴_0` :!via `PlayFromStart`)
        (:`Update`
          (`TimelineComponent.SetPlayRate` (`self.时间轴_1`) `_新建轨道_0`))))
    (:`then_3`
      (`KismetSystemLibrary.Delay` 2.0)
      (`self.Boom_CE`))))

(event `Boom_CE`
  (`self.SetActorEnableCollision` false)
  (for _array_element (`self.All`)
    (`self.K2_DetachFromActor` _array_element "KeepWorld" "KeepWorld" "KeepWorld")
    (`/Game/BP/爆炸球/BP_ballZs.FlyZ` _array_element (- (`SceneComponent.K2_GetComponentLocation` (`self.Arrow`)) (0.0 0.0 0.0))))
  (`ActorComponent.SetActive` (`self.P_Explosion`) true true)
  (`InstancedStaticMeshComponent.ClearInstances` (`self.HierarchicalInstancedStaticMesh`))
  (`KismetSystemLibrary.Delay` 2.0)
  (`SceneComponent.SetHiddenInGame` (`self.P_Explosion`) true false))

(event `self.Sphere外圈.OnComponentBeginOverlap`
  (params (OverlappedComponent :type "PrimitiveComponent Object Reference") (OtherActor :type "Actor Object Reference") (OtherComp :type "PrimitiveComponent Object Reference") (OtherBodyIndex :type Integer) (bFromSweep :type Boolean) (SweepResult :type "HitResult Structure (by ref)")))

(event `self.Sphere外圈.OnComponentEndOverlap`
  (params (OverlappedComponent :type "PrimitiveComponent Object Reference") (OtherActor :type "Actor Object Reference") (OtherComp :type "PrimitiveComponent Object Reference") (OtherBodyIndex :type Integer)))

(fn `UserConstructionScript`
  (for _ (range 501)
    _))