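; Exploding-ball (爆炸球) character that gets knocked away from a point, then walks back to it.
; Non-boss instances pick a random skeletal mesh with matching animation and scale, starting without collision.
; FlyZ enables collision and launches away from LaunchVelocity, actually a world position; OnLaunched plays the death animation.
; OnLanded waits, restores animation and Pawn blocking, then AI-moves toward that point; ragdoll and timed-destroy chains are disconnected.
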(event `self.ReceiveBeginPlay`
  (bind _mesh (`self.Mesh`))
  (bind _all_sk (`self.All_SK`))
  (`self.SetActorEnableCollision` false)
  (set `self.Index_SK` (`KismetMathLibrary.RandomIntegerInRange` 0 (`KismetArrayLibrary.Array_LastIndex` _all_sk)))
  (if (not (`self.Boss`))
    (`SkinnedMeshComponent.SetSkinnedAssetAndUpdate` _mesh (`|GetArrayItem` _all_sk (`self.Index_SK`)) true)
    (`SkeletalMeshComponent.PlayAnimation` _mesh (`|GetArrayItem` (`self.All_Anim`) (`self.Index_SK`)) true)
    (`SceneComponent.SetRelativeScale3D` (`self.Mesh`) (`|GetArrayItem` (`self.Scale_0`) (`self.Index_SK`)))))

(event `FlyZ`
  (params (LaunchVelocity :type "Vector Structure"))
  (bind _output_get (set `self.Launch Velocity` LaunchVelocity))
  (set `CharacterMovementComponent.GravityScale` 1.0 (`self.CharacterMovement`))
  (`self.SetActorEnableCollision` true)
  (bind _returnvalue (`KismetMathLibrary.Normal` (- (`self.K2_GetActorLocation`) _output_get)))
  (set `self.NewVar_0` _returnvalue)
  (bind (_returnvalue_x _returnvalue_y _returnvalue_z) (`KismetMathLibrary.BreakVector` (* _returnvalue (600.0 600.0 800.0))))
  (`self.LaunchCharacter` (`KismetMathLibrary.MakeVector` _returnvalue_x _returnvalue_y _returnvalue_z) true true) ; 1000
)

(event `self.OnLanded`
  (params (Hit :type "HitResult Structure (by ref)"))
  (`KismetSystemLibrary.PrintString` "Hello11111" true true (struct :`G` 0.66 :`B` 1.0 :`A` 1.0) 5.0)
  (`KismetSystemLibrary.Delay` 2.0)
  (`SkeletalMeshComponent.PlayAnimation` (`self.Mesh`) (`|GetArrayItem` (`self.All_Anim`) (`self.Index_SK`)) true)
  (`PrimitiveComponent.SetCollisionResponseToChannel` (`self.CapsuleComponent`) "ECC_Pawn" "ECR_Block")
  (`self.K2_SetActorRotation` (struct))
  (`|AIMoveTo` self (`KismetMathLibrary.MakeVector` (.x (`self.Launch Velocity`)) (.y (`self.Launch Velocity`)) 45.0) null 5.0 true))

(event `self.OnLaunched`
  (params (LaunchVelocity :type "Vector Structure") (bXYOverride :type Boolean) (bZOverride :type Boolean))
  (`KismetSystemLibrary.PrintString` "Hello32222" true true (struct :`G` 0.66 :`B` 1.0 :`A` 1.0) 5.0)
  (`SkeletalMeshComponent.PlayAnimation` (`self.Mesh`) (`|GetArrayItem` (`self.Die_Anim`) (`self.Index_SK`)) false))

(fn `UserConstructionScript`)