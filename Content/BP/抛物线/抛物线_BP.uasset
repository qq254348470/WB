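; Parabolic arc actor (抛物线_BP) that draws an animated projectile-style line from its Arrow toward an end point, starting at BeginPlay.
; A timeline extends the end point while Tick predicts the trajectory and bends pre-built spline meshes along it, with a debug arrow at impact.
; Near completion it moves PointBP to the impact and starts that actor's draw.
; Separate events retarget the arc to a hardcoded position or hide segments sequentially by timer.
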(event `StartDraw_CS`
  (bind _point_bp (`self.Point_BP`))
  (set `self.Condition` true)
  (bind (_direction `_新建轨道_0`) (`Timeline|时间轴_0` :!via `PlayFromStart`)
    (:`Update`
      (set `self.EndPoint_0` (`KismetMathLibrary.VLerp` (/ (`self.EndPoint`) 100.0) (`self.EndPoint`) `_新建轨道_0`))
      (if (>= `_新建轨道_0` 0.85)
        (`/Engine/EditorBlueprintResources/StandardMacros.IsValid` _point_bp
          (:`Is Valid`
            (`self.K2_SetActorLocation` _point_bp (+ (`self.Out Last Trace Destination`) (0.0 0.0 10.0)) false false)
            (`self.StartDraw_CS` _point_bp)))))))

(event `self.ReceiveBeginPlay`
  (`self.StartDraw_CS`)
  (`/Engine/EditorBlueprintResources/StandardMacros.IsValid` (`self.Point_BP`)
    (:`Is Valid`
      (`TimelineComponent.SetPlayRate` (`self.时间轴_0`) (`self.Rate`)))))

(event `self.ReceiveTick`
  (params (DeltaSeconds :type "Float (single-precision)"))
  (if (`self.Condition`)
    (`self.DrawPath_CS` (`self.EndPoint_0`))))

(event `Update_CS`
  (set `self.Condition` false)
  (`/Engine/EditorBlueprintResources/StandardMacros.DoOnce` false
    (:`Completed`
      (bind (_direction `_新建轨道_0`) (`Timeline|时间轴_1`)
        (:`Update`
          (`self.DrawPath_CS` (`KismetMathLibrary.VLerp` (`self.EndPoint`) (1400.0 -20.057129 -490.879883) `_新建轨道_0`)))))))

(event `DrawPath_CS`
  (params (A :type "Vector Structure"))
  (bind _arcspline (`self.ArcSpline`))
  (bind _splinemeshes (`self.SplineMeshes`))
  (bind _arcspline_2 (`self.ArcSpline`))
  (bind _returnvalue (`SceneComponent.K2_GetComponentLocation` (`self.Arrow`)))
  (bind _outlaunchvelocity (`GameplayStatics.SuggestProjectileVelocity_CustomArc` _returnvalue (+ (`KismetMathLibrary.GreaterGreater_VectorRotator` A (`self.K2_GetActorRotation`)) (`self.K2_GetActorLocation`)) (`self.Override Gravity Z`) (`self.Arc Param`)))
  (bind (_outhit _outpathpositions _outlasttracedestination _returnvalue_2) (`GameplayStatics.Blueprint_PredictProjectilePath_ByObjectType` :`StartPos` _returnvalue :`LaunchVelocity` _outlaunchvelocity :`ObjectTypes` (`|MakeArray` "ObjectTypeQuery1" :!type "EObjectTypeQuery Enum") :`bTraceComplex` true :`SimFrequency` 20.0 :`MaxSimTime` 5.0)) ; Simulate throwing a projectile (including gravity) to find a teleport location.
  (if _returnvalue_2
    (`|ExecutionSequence`
      (:`then_0`
        (`SplineComponent.ClearSplinePoints` _arcspline_2 true)
        (for _array_element (`self.SplineMeshes`)
          (`SplineMeshComponent.SetStartAndEnd` _array_element (0.0 0.0 0.0) (0.0 0.0 0.0) (0.0 0.0 0.0) (0.0 0.0 0.0) true) ; Set the tangents and position to build slightly bend the cylinder. All cylinders combined create a smooth arc.
        )
        (for _array_element_2 _outpathpositions
          (`SplineComponent.AddSplinePoint` _arcspline_2 _array_element_2 "World" true) ; Build a spline from all trace points. This generates tangets we can use to build a smoothly curved spline mesh
        )
        (`SplineComponent.SetSplinePointType` _arcspline_2 (`KismetArrayLibrary.Array_LastIndex` _outpathpositions) "CurveClamped" true) ; Update the point type to create the curve
        (for _index (range (+ (- (`SplineComponent.GetNumberOfSplinePoints` (`self.ArcSpline`)) 2) 1))
          (if (<= _index (`KismetArrayLibrary.Array_LastIndex` _splinemeshes))
            (bind _returnvalue_3 (+ _index 1))
            (`SplineMeshComponent.SetStartAndEnd` (`|GetArrayItem` _splinemeshes _index) (`|GetArrayItem` _outpathpositions _index) (`SplineComponent.GetTangentAtSplinePoint` _arcspline _index "Local") (`|GetArrayItem` _outpathpositions _returnvalue_3) (`SplineComponent.GetTangentAtSplinePoint` _arcspline _returnvalue_3 "Local") true) ; Set the tangents and position to build slightly bend the cylinder. All cylinders combined create a smooth arc.
          )))
      (:`then_2`
        (bind _output_get (set `self.Out Last Trace Destination` (`|GetArrayItem` _outpathpositions (`KismetArrayLibrary.Array_LastIndex` _outpathpositions))))
        (`KismetSystemLibrary.DrawDebugArrow` _output_get (+ _output_get (0.0 0.0 55.0)) 10.0 (struct :`R` 1.0 :`A` 1.0) 5.0 10.0)))))

(event `StartShow_CS`
  (`KismetSystemLibrary.K2_SetTimerDelegate` (delegate `Show_CS`) (`self.Time`) true))

(event `Show_CS`
  (bind _splinemeshes (`self.SplineMeshes`))
  (`SceneComponent.SetVisibility` (`|GetArrayItem` _splinemeshes (`KismetMathLibrary.Clamp` (`self.NewVar_2`) 0 (`KismetArrayLibrary.Array_LastIndex` _splinemeshes))) false false)
  (`/Engine/EditorBlueprintResources/StandardMacros.IncrementInt` (`self.NewVar_2`)))

(fn `UserConstructionScript`
  (bind _splinemeshes (`self.SplineMeshes`))
  (for _array_element _splinemeshes
    (`ActorComponent.K2_DestroyComponent` _array_element))
  (`KismetArrayLibrary.Array_Clear` _splinemeshes)
  (for _ (range 56)
    (bind _returnvalue (`AddComponent|NODE_AddSplineMeshComponent-1` :`bManualAttachment` true :`RelativeTransform` (`KismetMathLibrary.MakeTransform` (0.0 0.0 0.0)))) ; Add new cylinder mesh
    (`KismetArrayLibrary.Array_Add` (`self.SplineMeshes`) _returnvalue)))