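; Climbing AI character for a human-ladder crowd, which climbs along a spline and then falls off as a ragdoll.
; BeginPlay picks a random mesh and play rate, then a timeline moves the actor along the spline, keeping its starting offset, and unhides it shortly after.
; When the timeline finishes, death launches the character backward, switches to physics ragdoll and destroys it after a random delay.
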(event `self.ReceiveBeginPlay`
  (bind `_模型` (`self.模型`))
  (`|ExecutionSequence`
    (:`then_0`
      (`SkinnedMeshComponent.SetSkinnedAssetAndUpdate` (`self.Mesh`) (`|GetArrayItem` `_模型` (`KismetMathLibrary.RandomIntegerInRange` 0 (`KismetArrayLibrary.Array_LastIndex` `_模型`))) true)
      (`TimelineComponent.SetPlayRate` (`self.时间轴_0`) (`KismetMathLibrary.RandomFloatInRange` 4.4 4.7))
      (set `self.Offset` (- (`self.K2_GetActorLocation`) (`self.K2_GetActorLocation` (`self.ASpline`))))
      (bind (_direction `_新建轨道_0`) (`Timeline|时间轴_0` :!via `PlayFromStart`)
        (:`Update`
          (bind _returnvalue (`/Game/BP/爬人梯/AI_Spline.World_CS` (`self.ASpline`) `_新建轨道_0`))
          (`self.K2_SetActorTransform` (`KismetMathLibrary.MakeTransform` (+ (.location _returnvalue) (`self.Offset`)) (`KismetMathLibrary.MakeRotator` 0.0 0.0 (.yaw (.rotation _returnvalue))) (.scale _returnvalue)))
          (if (>= `_新建轨道_0` (`KismetMathLibrary.RandomFloatInRange` 0.7 1.0))
            _))
        (:`Finished`
          (`self.Die_CS`))))
    (:`then_1`
      (`KismetSystemLibrary.Delay` 0.2)
      (`self.SetActorHiddenInGame` false))))

(event `Die_CS`
  (bind _mesh (`self.Mesh`))
  (if (not (`self.Die`))
    (`self.SetActorEnableCollision` false)
    (set `self.Die` true)
    (`TimelineComponent.Stop` (`self.时间轴_0`))
    (`MovementComponent.StopMovementImmediately` (`self.CharacterMovement`))
    (`self.LaunchCharacter` (+ (* (`SceneComponent.GetForwardVector` (`self.ArrowComponent`)) -150.0) (0.0 0.0 100.0)) true true) ; 1000
    (`KismetSystemLibrary.Delay` 0.3)
    (`SkeletalMeshComponent.SetAllBodiesSimulatePhysics` _mesh true)
    (`SkeletalMeshComponent.SetAllBodiesPhysicsBlendWeight` _mesh 1.0 true)
    (`PrimitiveComponent.SetCollisionEnabled` _mesh "QueryAndPhysics")
    (`PrimitiveComponent.SetCollisionEnabled` (`self.CapsuleComponent`) "NoCollision")
    (`|ExecutionSequence`
      (:`then_0`
        (`KismetSystemLibrary.Delay` (`KismetMathLibrary.RandomFloatInRange` 3.0 5.0))
        (`self.K2_DestroyActor`))
      (:`then_1`
        (`KismetSystemLibrary.Delay` 0.8)
        (`self.SetActorEnableCollision` true)))))

(fn `UserConstructionScript`)