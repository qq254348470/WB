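; Wild-monster AI child Blueprint handling waypoints, health, hit reactions and death.
; Picks its next NewPoint from the AImoveToSpline array or a random navmesh point near spawn, advancing when within range; the timeline spline mover is disconnected.
; Interface damage reduces HP until death, while range triggers slow it or briefly freeze it with an ice material.
; Fly knockback kills non-bosses via launch, material fade and ragdoll before destruction.
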(event `UpdateIndex_CS`
  (bind _aimovetospline (`self.AImoveToSpline`))
  (`KismetSystemLibrary.Delay` 0.0)
  (if (`self.Random`)
    (bind _output_get (set `self.NewPoint` (`NavigationSystemV1.K2_GetRandomReachablePointInRadius` (`NavigationSystemV1.GetNavigationSystem`) (`self.StartLocation`) 500.0 null "/Game/创世之争/野怪/AI/CS_NavFilter.CS_NavFilter_C")))
    (`KismetSystemLibrary.DrawDebugSphere` _output_get 15.0 12 (struct :`R` 1.0 :`A` 1.0) 1.0 3.0)
    (set `CharacterMovementComponent.MaxWalkSpeed` 20.0 (`self.CharacterMovement`))
    (`/Engine/EditorBlueprintResources/StandardMacros.DoOnce` false
      (:`Completed`
        (`KismetSystemLibrary.Delay` 5.0)
        (set `self.Random` false)
        (set `CharacterMovementComponent.MaxWalkSpeed` 600.0 (`self.CharacterMovement`))))
    (else
      (bind _output_get_2 (set `self.Index` (+ (`self.Index`) 1)))
      (if (>= _output_get_2 (`KismetArrayLibrary.Array_Length` _aimovetospline))
        (set `self.Index` -1)
        (else
          (set `self.NewPoint` (`/Game/创世之争/野怪/BP/ASpline_BP.GetDistancePoint_CF` (`|GetArrayItem` _aimovetospline (`self.Index`)) (`self.Distance`))))))))

(event `self.ReceiveBeginPlay`
  (`|ExecutionSequence`
    (:`then_0`
      (`self.InitInfo_CS`))
    (:`then_1`
      (`self.BossSetting_CS`))
    (:`then_2`
      (`KismetSystemLibrary.Delay` 0.0)
      (`self.MoveSetting_CS` 5.0) ; 0.8
    )
    (:`then_3`)))

(event `CheckPoint_CS`
  (if (<= (`KismetMathLibrary.VSize` (- (`self.K2_GetActorLocation`) (`self.NewPoint`))) 150.0)
    (`self.UpdateIndex_CS`)))

(event `InitInfo_CS`
  (`self.ChangeM_CF` true) ; 记录初始材质
  (set `self.StartLocation` (`self.K2_GetActorLocation`))
  (cast `/Game/创世之争/野怪/AI/HP_UMG` (`WidgetComponent.GetUserWidgetObject` (`self.HP`))))

(event `BossSetting_CS`
  (`SceneComponent.SetVisibility` (`self.HP`) true false)
  (set `self.MaxHP` (`self.CurrentHP`)))

(event `MoveSetting_CS`
  (params (Rate :type "Float (double-precision)")))

(event `ChangeRate_CS`
  (params (Range :type Boolean))
  (bind _charactermovement (`self.CharacterMovement`))
  ;[1 1 1] 范围内减速
  (if Range
    (`/Engine/EditorBlueprintResources/StandardMacros.DoOnce` false :!label _label
      (:`Completed`
        (bind (_direction _changespeed) (`Timeline|时间轴_2` :!via `PlayFromStart`)
          (:`Update`
            (set `CharacterMovementComponent.MaxWalkSpeed` (`KismetMathLibrary.Lerp` 800.0 400.0 _changespeed) _charactermovement)))))
    (else
      (set `CharacterMovementComponent.MaxWalkSpeed` 800.0 _charactermovement)
      (goto _label :!via `Reset`))))

(event `HitDamage_CS`
  (params (Damage :type "Float (double-precision)"))
  (bind _returnvalue (`self.Damage_CF` Damage))
  (if _returnvalue
    (set `self.Die` true)
    (if (`self.Boss`)
      (`TimelineComponent.Stop` (`self.时间轴_移动`))
      (`self.SetActorEnableCollision` false)
      (else
        (`self.SetActorEnableCollision` false)
        (`TimelineComponent.Stop` (`self.时间轴_移动`))
        (`NavMovementComponent.StopActiveMovement` (`self.CharacterMovement`))
        (`KismetSystemLibrary.Delay` (`KismetMathLibrary.RandomFloatInRange` 2.0 4.0))
        (`self.K2_DestroyActor`)))))

(event `/Game/创世之争/野怪/BP/CSAI_Interface.CSIF_AI_Damage`
  (params (Damage :type "Float (single-precision)"))
  (if (> (`self.CurrentHP`) 0.0)
    (`self.HitDamage_CS` Damage)))

(event `UpdateM_CS`
  (bind _dy_m (`self.Dy_M`))
  (`/Engine/EditorBlueprintResources/StandardMacros.IsValid` _dy_m
    (:`Is Valid`
      (`/Engine/EditorBlueprintResources/StandardMacros.DoOnce` false
        (:`Completed`
          (`MaterialInstanceDynamic.SetScalarParameterValue` (`self.Dy_M`) "Hit" 1.0)
          (`PrimitiveComponent.SetMaterial` (`self.Mesh`) 0 _dy_m)
          (`TimelineComponent.SetPlayRate` (`self.时间轴_0`) 0.5)
          (bind (_direction `_新建轨道_0`) (`Timeline|时间轴_0` :!via `PlayFromStart`)
            (:`Update`
              (`MaterialInstanceDynamic.SetScalarParameterValue` (`self.Dy_M`) "Alpha" `_新建轨道_0`))
            (:`Finished`
              (`self.K2_DestroyActor`))))))))

(event `InRange_CS`
  (params (In :type Boolean))
  (if In
    (`/Engine/EditorBlueprintResources/StandardMacros.DoOnce` false :!label _label_2
      (:`Completed`
        (for (_ _array_index) (`self.Mesh_Materials`)
          (`PrimitiveComponent.SetMaterial` (`self.Mesh`) _array_index "/Game/创世之争/母材质/冰冻/Ice_m_Inst.Ice_m_Inst"))
        (`TimelineComponent.Stop` (`self.时间轴_移动`))
        (set `self.MoveRate_Animation` 0.0)
        (`KismetSystemLibrary.Delay` 2.0)
        (if (not (`self.Die`))
          (`TimelineComponent.Play` (`self.时间轴_移动`))
          (`self.ChangeM_CF` false)
          (set `self.MoveRate_Animation` 1.0)
          (`self.Rest_CS`))))))

(event `Rest_CS`
  (goto _label_2 :!via `Reset`))

(event `Debuff_Par`
  (bind _debuff (`self.Debuff`))
  (`ActorComponent.SetActive` _debuff true false)
  (`KismetSystemLibrary.Delay` (`KismetMathLibrary.RandomFloatInRange` 0.05 0.1))
  (`ActorComponent.SetActive` _debuff false false))

(event `Hit_Par_CS`
  (bind _hit_par (`self.Hit_Par`))
  (`ActorComponent.SetActive` _hit_par true false)
  (`KismetSystemLibrary.Delay` (`KismetMathLibrary.RandomFloatInRange` 0.05 0.1))
  (`ActorComponent.SetActive` _hit_par false false))

(event `Fly_CS`
  (params (Point :type "Vector Structure") (Speed :type "Vector Structure" :default (300.0 300.0 300.0)))
  (bind _mesh (`self.Mesh`))
  (bind (_returnvalue_x _returnvalue_y) (`KismetMathLibrary.BreakVector` (* (`KismetMathLibrary.Normal` (- (`self.K2_GetActorLocation`) Point)) Speed)))
  (if (`self.Boss`)
    _
    (elif (not (`self.Die`))
      (set `self.Die` true)
      (`TimelineComponent.Stop` (`self.时间轴_移动`))
      (`MovementComponent.StopMovementImmediately` (`self.CharacterMovement`))
      (`self.LaunchCharacter` (`KismetMathLibrary.MakeVector` _returnvalue_x _returnvalue_y (.z Speed)) true true) ; 1000
      (`self.UpdateM_CS`)
      (`KismetSystemLibrary.Delay` 0.1) ; 0.3
      (`SkeletalMeshComponent.SetAllBodiesSimulatePhysics` _mesh true)
      (`SkeletalMeshComponent.SetAllBodiesPhysicsBlendWeight` _mesh 1.0 true)
      (`PrimitiveComponent.SetCollisionEnabled` _mesh "QueryAndPhysics")
      (`PrimitiveComponent.SetCollisionEnabled` (`self.CapsuleComponent`) "NoCollision")
      (`KismetSystemLibrary.Delay` (`KismetMathLibrary.RandomFloatInRange` 3.0 5.0))
      (`self.K2_DestroyActor`))))

(event `/Game/创世之争/野怪/BP/CSAI_Interface.CSIF_AI_Fly`
  (params (Point :type "Vector Structure") (Speed :type "Vector Structure"))
  (`self.Fly_CS` Point Speed))

(fn `ChangeM_CF`
  (params (SaveMaterials :type Boolean)))

(fn `Damage_CF`
  (params (Damage :type "Float (double-precision)"))
  (returns (ReturnValue :type Boolean))
  (bind _output_get (set `self.CurrentHP` (- (`self.CurrentHP`) Damage)))
  (return (<= (/ _output_get (`self.MaxHP`)) 0.02)))

(fn `UserConstructionScript`
  (`parent.UserConstructionScript`)
  (bind _returnvalue (`KismetMaterialLibrary.CreateDynamicMaterialInstance` (`PrimitiveComponent.GetMaterial` (`self.Mesh`) 0)))
  (set `self.Dy_M` _returnvalue))