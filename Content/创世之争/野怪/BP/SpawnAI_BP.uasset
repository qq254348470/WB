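; SpawnAI_BP is a spawner actor that creates waves of wild monsters and hands each one spline paths to move along.
; If enabled, it waits on BeginPlay, then loops a timer and pauses it after a fixed period; StartSpawn_CS also starts this, and End_CS clears it.
; Each wave spreads the selected class along a grid-snapped, rotated box or the first path spline.
; A SpawnBoss event spawns a 独眼_BP, but its timer setup is disconnected.
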(event `End_CS`
  (`KismetSystemLibrary.K2_ClearAndInvalidateTimerHandle` (`self.Timer`))
  (`KismetSystemLibrary.K2_ClearAndInvalidateTimerHandle` (`self.TimerBoss`)))

(event `SpawnBoss`
  (bind (_returnvalue_x _returnvalue_y) (`KismetMathLibrary.BreakVector` (`BoxComponent.GetScaledBoxExtent` (`self.Box`))))
  (bind _returnvalue (+ (`KismetMathLibrary.GreaterGreater_VectorRotator` (`KismetMathLibrary.MakeVector` (+ (`KismetMathLibrary.Lerp` _returnvalue_x (* _returnvalue_x -1.0) 0.5) 1.0) (+ (`KismetMathLibrary.RandomFloatInRange` (* _returnvalue_y -1.0) _returnvalue_y) 1.0)) (`self.K2_GetActorRotation`)) (`self.K2_GetActorLocation`)))
  (for _ (range 1)
    (`|SpawnActorFromClass` "/Game/创世之争/野怪/duyanjuren/独眼_BP.独眼_BP_C" (`KismetMathLibrary.MakeTransform` _returnvalue) "AlwaysSpawn" "OverrideRootScale" null (`self.Spline`) _returnvalue (`/Game/创世之争/野怪/BP/PathSpline_BP.TargetAll` (`self.PathSpline_BP`)) 0.5 null)))

(event `self.ReceiveBeginPlay`
  (if (`self.Can`)
    (`KismetSystemLibrary.Delay` (`self.DelayTime`)) ; 3
    (bind _returnvalue (`KismetSystemLibrary.K2_SetTimerDelegate` (delegate `SpawnAI`) 0.5 true :!label _label)) ; 1
    (bind _output_get (set `self.Timer` _returnvalue))
    (`KismetSystemLibrary.Delay` 50.0)
    (`KismetSystemLibrary.K2_PauseTimerHandle` _output_get)))

(event `StartSpawn_CS`
  (goto _label))

(event `SpawnAI`
  (bind (_returnvalue_x _returnvalue_y) (`KismetMathLibrary.BreakVector` (`BoxComponent.GetScaledBoxExtent` (`self.Box`))))
  (for _ (range (+ (`self.Num`) 1))
    (bind _output_get (set `self.Distance` (mod (+ (`self.Distance`) (/ 1.0 (`KismetMathLibrary.Conv_IntToDouble` (`self.Num`)))) 1.0)))
    (bind _output_get_2 (set `self.Point` (select `bool` (`self.AsBoxSpawn`) :`false` (`/Game/创世之争/野怪/BP/ASpline_BP.GetDistancePoint_CF` (`|GetArrayItem` (`/Game/创世之争/野怪/BP/PathSpline_BP.TargetAll` (`self.PathSpline_BP`))) _output_get) :`true` (+ (`KismetMathLibrary.GreaterGreater_VectorRotator` (`KismetMathLibrary.MakeVector` (+ (* (`.ReturnValue` (`KismetMathLibrary.FMod` (`KismetMathLibrary.Lerp` _returnvalue_x (* _returnvalue_x -1.0) (`self.Distance`)) 80.0)) 80.0) 1.0) (+ (* (`.ReturnValue` (`KismetMathLibrary.FMod` (`KismetMathLibrary.RandomFloatInRange` (* _returnvalue_y -1.0) _returnvalue_y) 30.0)) 30.0) 1.0)) (`self.K2_GetActorRotation`)) (`self.K2_GetActorLocation`)))))
    (`|SpawnActorFromClass` (`|GetArrayItem` (`self.野怪Child_BP`) (`self.指定怪物`)) (`KismetMathLibrary.MakeTransform` _output_get_2 (struct :`Yaw` 270.0) (0.7 0.7 0.7)) "AlwaysSpawn" "OverrideRootScale" null (`self.Spline`) _output_get_2 (`/Game/创世之争/野怪/BP/PathSpline_BP.TargetAll` (`self.PathSpline_BP`)) (`self.Distance`) null)))

(fn `UserConstructionScript`)