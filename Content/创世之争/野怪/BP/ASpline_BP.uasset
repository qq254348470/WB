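; ASpline_BP is a spline helper actor, filed under wild monsters, that supplies positions and transforms along a path.
; Its construction script places a child actor at each spline point and caches them in AsArrowPointBP.
; Query functions take normalized distances, with a yaw offset on transforms, and GetTargetDistancePoints also spawns child actors at evenly spaced samples.
; UpdatePointCF reshapes the spline into a centered two-point line along local Y, scaled by its input.
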(fn `GetDistancePoint_CF`
  (params (NewParam :type "Float (double-precision)"))
  (returns (Point :type "Vector Structure"))
  (bind _spline (`self.Spline`))
  (return (`SplineComponent.GetLocationAtDistanceAlongSpline` _spline (* NewParam (`SplineComponent.GetSplineLength` _spline)) "World")))

(fn `GetLength_CF`
  (returns (ReturnValue :type "Float (double-precision)"))
  (return (`SplineComponent.GetSplineLength` (`self.Spline`))))

(fn `GetPointLocation_CF`
  (params (PointIndex :type Integer))
  (returns (`Return Value Location` :type "Vector Structure"))
  (bind _returnvalue_location (`KismetMathLibrary.BreakTransform` (`SplineComponent.GetTransformAtSplinePoint` (`self.Spline`) PointIndex "World" false)))
  (return _returnvalue_location))

(fn `GetTargetDistancePoints_CF`
  (params (Num :type Integer))
  (returns (NewLocalVar_01 :type "Array of Transform Structure"))
  (locals (NewLocalVar_0 :type "Array of Transform Structure"))
  (bind _returnvalue (- Num 1))
  (bind _newlocalvar_0 (`local.NewLocalVar_0`))
  (for _index (range (+ _returnvalue 1))
    (bind _newparam (`self.GetWorldPoint_CF` (* _index (/ 1.0 (`KismetMathLibrary.Conv_IntToDouble` _returnvalue)))))
    (`KismetArrayLibrary.Array_Add` _newlocalvar_0 _newparam)
    (bind _returnvalue_2 (`AddComponent|NODE_AddChildActorComponent-1` :`bManualAttachment` true))
    (`SceneComponent.K2_SetWorldTransform` _returnvalue_2 _newparam false false))
  (return _newlocalvar_0))

(fn `GetWorldPoint_CF`
  (params (Distance :type "Float (double-precision)"))
  (returns (NewParam :type "Transform Structure"))
  (bind _spline (`self.Spline`))
  (return (`KismetMathLibrary.MakeTransform` (.location (`SplineComponent.GetTransformAtDistanceAlongSpline` _spline (* Distance (`SplineComponent.GetSplineLength` _spline)) "World" false)) (`KismetMathLibrary.MakeRotator` (.roll (.rotation (`SplineComponent.GetTransformAtDistanceAlongSpline` _spline (* Distance (`SplineComponent.GetSplineLength` _spline)) "World" false))) (.pitch (.rotation (`SplineComponent.GetTransformAtDistanceAlongSpline` _spline (* Distance (`SplineComponent.GetSplineLength` _spline)) "World" false))) (+ (.yaw (.rotation (`SplineComponent.GetTransformAtDistanceAlongSpline` _spline (* Distance (`SplineComponent.GetSplineLength` _spline)) "World" false))) (`self.左右偏移`))) (.scale (`SplineComponent.GetTransformAtDistanceAlongSpline` _spline (* Distance (`SplineComponent.GetSplineLength` _spline)) "World" false)))))

(fn `Update Point CF`
  (params (A :type "Vector Structure"))
  (`SplineComponent.SetSplinePoints` (`self.Spline`) (`|MakeArray` (* A (0.0 -100.0 0.0)) (* A (0.0 100.0 0.0))) "Local" true))

(fn `UserConstructionScript`
  (bind _spline (`self.Spline`))
  (`KismetArrayLibrary.Array_Clear` (`self.As Arrow Point BP`))
  (for _index (range (`SplineComponent.GetNumberOfSplinePoints` _spline))
    (bind _returnvalue (`AddComponent|NODE_AddChildActorComponent-0` :`RelativeTransform` (`KismetMathLibrary.Conv_VectorToTransform` (`SplineComponent.GetLocationAndTangentAtSplinePoint` _spline _index "Local"))))
    (`KismetArrayLibrary.Array_Add` (`self.As Arrow Point BP`) (`ChildActorComponent.ChildActor` _returnvalue))))