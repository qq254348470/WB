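; Electromagnetic tower (电磁塔) that spins and periodically zaps zombies (丧尸_BP) in its range.
; After a scale-up timeline, a looping timer fires pooled beam particles, built in the construction script, at zombies tracked by sphere overlaps.
; Each hit launches nearby zombies via FlyCS; the direct damage call is disconnected.
; Tick calls ChangeRateCS on zombies inside the sphere, and Clear_CS starts rapid strikes across the Fanweiquan area.
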(event `self.ReceiveTick`
  (params (DeltaSeconds :type "Float (single-precision)"))
  (if (`self.True`)
    (`|ExecutionSequence`
      (:`then_0`
        (`SceneComponent.K2_AddRelativeRotation` (`self.Mesh`) (struct :`Yaw` 12.0) false false))
      (:`then_1`
        (for _array_element (`PrimitiveComponent.GetOverlappingActors` (`self.Sphere`) "/Game/创世之争/野怪/丧尸/丧尸_BP.丧尸_BP_C")
          (bind `_as丧尸_bp` (cast `/Game/创世之争/野怪/丧尸/丧尸_BP` _array_element))
          (`/Game/创世之争/野怪/丧尸/丧尸_BP.ChangeRate_CS` `_as丧尸_bp` false))))))

(event `self.ReceiveBeginPlay`
  (`ActorComponent.SetActive` (`self.0`) true false)
  (`SceneComponent.SetRelativeScale3D` (`self.Mesh`) (0.0 0.0 0.0))
  (`SceneComponent.SetRelativeScale3D` (`self.P_hudun_2`) (0.0 0.0 0.0))
  (`ActorComponent.SetActive` (`self.0`) true false)
  (`KismetSystemLibrary.Delay` 0.5)
  (`self.Init_CS`)
  (`KismetSystemLibrary.Delay` 3.0))

(event `Init_CS`
  ;[1 1 1] 注释
  (bind (_direction `_新建轨道_0`) (`Timeline|时间轴_0` :!via `PlayFromStart`)
    (:`Update`
      (`SceneComponent.SetRelativeScale3D` (`self.Mesh`) (`KismetMathLibrary.Conv_DoubleToVector` (* `_新建轨道_0` (`self.Scale`))))
      (`SceneComponent.SetRelativeScale3D` (`self.P_hudun_2`) (`KismetMathLibrary.Conv_DoubleToVector` (* `_新建轨道_0` 1.0))))
    (:`Finished`
      (set `self.True` true)
      (`KismetSystemLibrary.K2_SetTimerDelegate` (delegate `FindTarget_CS`) (`self.CD`) true))))

(event `FindTarget_CS`
  (bind _as_ai_bp (`self.As AI BP`))
  (bind _returnvalue (`KismetArrayLibrary.Array_LastIndex` _as_ai_bp))
  (`ActorComponent.SetActive` (`self.Hit_Start`) false false)
  (for _array_element (`self.ParticleCom`)
    (`ActorComponent.SetActive` _array_element false false))
  (if (>= _returnvalue 0)
    (for (_array_element_2 _array_index) (`self.ParticleCom`)
      (if (<= _array_index _returnvalue)
        (bind _output (`|GetArrayItem` _as_ai_bp _array_index))
        (if (not (`/Game/创世之争/野怪/AI/野怪Parent_BP.Die` _output))
          (`self.Hit_CS` _array_element_2 _output))))
    (`KismetSystemLibrary.Delay` 0.2)
    (for _array_element_3 (`self.ParticleCom`)
      (`ActorComponent.SetActive` _array_element_3 false true))))

(event `Clear_CS`
  (`KismetSystemLibrary.K2_SetTimerDelegate` (delegate `自定义事件_0`) 0.1 true)
  (set `self.Damage` (100.0 101.0)))

(event `自定义事件_0`
  (for (_array_element _array_index) (`PrimitiveComponent.GetOverlappingActors` (`self.fanweiquan`) "/Game/创世之争/野怪/丧尸/丧尸_BP.丧尸_BP_C")
    (`self.Hit_CS` (`|GetArrayItem` (`self.ParticleCom`) _array_index) _array_element)))

(event `Hit_CS`
  (params (Particle :type "FXSystemComponent Object Reference") (Actor :type "Actor Object Reference"))
  (`FXSystemComponent.SetActorParameter` Particle "Target" Actor)
  (`|ExecutionSequence`
    (:`then_0`
      (`ActorComponent.SetActive` Particle true true)
      (`ActorComponent.SetActive` (`self.Hit_Start`) true true))
    (:`then_1`
      (bind `_as丧尸_bp` (cast `/Game/创世之争/野怪/丧尸/丧尸_BP` Actor))
      (`|ExecutionSequence`
        (:`then_0`
          (`|MultiGate` false true (`self.Start Index`)
            (:`Out 2`
              (bind _returnvalue (`self.K2_GetActorLocation` `_as丧尸_bp`))
              (`GameplayStatics.SpawnEmitterAtLocation` "/Game/Effect/Particles/P_强力电击_受击.P_强力电击_受击" _returnvalue (struct) (0.1 0.1 0.1)))))
        (:`then_1`
          (bind _outactors (`KismetSystemLibrary.SphereOverlapActors` _returnvalue 50.0 (`|MakeArray` "ObjectTypeQuery3" :!type "EObjectTypeQuery Enum") "/Script/Engine.Actor"))
          (bind _output_get (set `self.Out Actors` _outactors))
          (if (> (`KismetArrayLibrary.Array_Length` _output_get) 0)
            (for (_array_element _array_index) _output_get
              (if (`self.Kill`)
                (bind `_as丧尸_bp_2` (cast `/Game/创世之争/野怪/丧尸/丧尸_BP` _array_element :!label _label))
                (`/Game/创世之争/野怪/丧尸/丧尸_BP.Fly_CS` `_as丧尸_bp_2` _returnvalue (300.0 300.0 300.0))
                (else
                  (set `self.CD` 0.5)
                  (if (<= _array_index 0)
                    (goto _label)))))))))))

(event `self.Sphere.OnComponentBeginOverlap`
  (params (OverlappedComponent :type "PrimitiveComponent Object Reference") (OtherActor :type "Actor Object Reference") (OtherComp :type "PrimitiveComponent Object Reference") (OtherBodyIndex :type Integer) (bFromSweep :type Boolean) (SweepResult :type "HitResult Structure (by ref)"))
  (bind `_as丧尸_bp` (cast `/Game/创世之争/野怪/丧尸/丧尸_BP` OtherActor))
  (`KismetArrayLibrary.Array_AddUnique` (`self.As AI BP`) `_as丧尸_bp`)
  (`/Engine/EditorBlueprintResources/StandardMacros.DoOnce` false
    (:`Completed`
      (set `self.Kill` true))))

(event `self.Sphere.OnComponentEndOverlap`
  (params (OverlappedComponent :type "PrimitiveComponent Object Reference") (OtherActor :type "Actor Object Reference") (OtherComp :type "PrimitiveComponent Object Reference") (OtherBodyIndex :type Integer))
  (bind `_as丧尸_bp` (cast `/Game/创世之争/野怪/丧尸/丧尸_BP` OtherActor))
  (`KismetArrayLibrary.Array_RemoveItem` (`self.As AI BP`) `_as丧尸_bp`))

(fn `CSIF_AI_State`
  (returns (Die :type Boolean) (Speed :type "Float (double-precision)"))
  (return false 0.0))

(fn `UserConstructionScript`
  (`KismetArrayLibrary.Array_Clear` (`self.ParticleCom`))
  (`SceneComponent.SetRelativeScale3D` (`self.Mesh`) (`KismetMathLibrary.Conv_DoubleToVector` (`self.Scale`)))
  (for _ (range 1 (+ (`self.Max`) 1))
    (bind _returnvalue (`AddComponent|NODE_AddParticleSystemComponent-1` :`bManualAttachment` true :`RelativeTransform` (`KismetMathLibrary.MakeTransform` (0.0 0.0 0.0) (struct) (0.030769 0.030769 0.030769))))
    (`KismetArrayLibrary.Array_Add` (`self.ParticleCom`) _returnvalue)
    (`SceneComponent.K2_AttachToComponent` _returnvalue (`self.Mesh`) "01" "KeepRelative" "KeepRelative" "KeepRelative" true)))