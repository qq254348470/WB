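; Damage actor for the level 1 laser turret that hurts zombies (丧尸_BP) inside its Sphere and toggles its hit particle effect.
; SetKill_CS or a zombie beginning overlap triggers a DoOnce-gated burst that briefly enables sphere queries, then sends damage to every overlapping zombie via CSIFAIDamageMessage.
; The Kill flag selects fixed heavy damage over a random product, and a shorter delay before the gate resets.
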(event `SetKill_CS`
  (params (Kill :type Boolean))
  (bind _sphere (`self.Sphere`))
  (set `self.Kill` Kill)
  (`/Engine/EditorBlueprintResources/StandardMacros.DoOnce` false :!label _label
    (:`Completed`
      (`PrimitiveComponent.SetCollisionEnabled` _sphere "QueryOnly")
      (for _array_element (`PrimitiveComponent.GetOverlappingActors` (`self.Sphere`) "/Game/创世之争/野怪/丧尸/丧尸_BP.丧尸_BP_C")
        (message `/Game/创世之争/野怪/BP/CSAI_Interface.CSIF_AI_Damage` _array_element (`KismetMathLibrary.SelectFloat` 100.0 (`KismetMathLibrary.Conv_IntToDouble` (* (`KismetMathLibrary.RandomIntegerInRange` 3 8) (`KismetMathLibrary.RandomIntegerInRange` 2 8))) (`self.Kill`))))
      (`PrimitiveComponent.SetCollisionEnabled` _sphere "NoCollision")
      (`KismetSystemLibrary.Delay` (`KismetMathLibrary.SelectFloat` 0.1 0.3 (`self.Kill`)))
      (goto _label :!via `Reset`))))

(event `ACFX_CS`
  (params (bNewActive :type Boolean) (bReset :type Boolean))
  (`ActorComponent.SetActive` (`self.P_jiguangpaoLV3_shouji_2`) bNewActive bReset))

(event `self.Sphere.OnComponentBeginOverlap`
  (params (OverlappedComponent :type "PrimitiveComponent Object Reference") (OtherActor :type "Actor Object Reference") (OtherComp :type "PrimitiveComponent Object Reference") (OtherBodyIndex :type Integer) (bFromSweep :type Boolean) (SweepResult :type "HitResult Structure (by ref)"))
  (cast `/Game/创世之争/野怪/丧尸/丧尸_BP` OtherActor)
  (goto _label))

(fn `UserConstructionScript`)