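; Level 1 laser turret that scales in on spawn, tracks zombies (丧尸_BP) entering its sphere, and fires a beam at one.
; Tick keeps the current target until it dies, then tries the first listed zombie, sleeping when the list is empty.
; The child damage actor, fed the Kill value, attaches to the target and serves as the beam particle's Target parameter, while the turret mesh yaws to follow.
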(event `self.ReceiveBeginPlay`
  (`|ExecutionSequence`
    (:`then_0`
      (bind `_as激光_damage_bp` (cast `/Game/创世之争/炮塔/激光/LV1/激光Damage_BP` (`ChildActorComponent.ChildActor` (`self.激光Damage_BP`))))
      (bind _output_get (set `self.FX` `_as激光_damage_bp`))
      (`/Game/创世之争/炮塔/激光/LV1/激光Damage_BP.SetKill_CS` _output_get (`self.Kill`)))
    (:`then_1`
      (bind (_direction `_新建轨道_0`) (`Timeline|时间轴_0` :!via `PlayFromStart`)
        (:`Update`
          (bind _output_get_2 (set `self.大小` `_新建轨道_0`))
          (`SceneComponent.SetRelativeScale3D` (`self.SM_激光炮LV1_攻击`) (`KismetMathLibrary.Conv_DoubleToVector` _output_get_2)))
        (:`Finished`
          (`self.SetActorTickEnabled` true))))))

(event `Start_CS`
  (`SceneComponent.SetVisibility` (`self.SM_激光炮LV1_攻击`) true false)
  (`KismetSystemLibrary.Delay` 0.0)
  (`SceneComponent.SetVisibility` (`self.P_jiguangpaoLV2`) true false)
  (`KismetSystemLibrary.Delay` 0.0)
  (`SceneComponent.SetVisibility` (`self.激光Damage_BP`) true true))

(event `self.Sphere.OnComponentBeginOverlap`
  (params (OverlappedComponent :type "PrimitiveComponent Object Reference") (OtherActor :type "Actor Object Reference") (OtherComp :type "PrimitiveComponent Object Reference") (OtherBodyIndex :type Integer) (bFromSweep :type Boolean) (SweepResult :type "HitResult Structure (by ref)"))
  (bind `_as丧尸_bp` (cast `/Game/创世之争/野怪/丧尸/丧尸_BP` OtherActor))
  (`KismetArrayLibrary.Array_AddUnique` (`self.As AI BP`) `_as丧尸_bp`)
  (`self.SetActorTickEnabled` true))

(event `self.Sphere.OnComponentEndOverlap`
  (params (OverlappedComponent :type "PrimitiveComponent Object Reference") (OtherActor :type "Actor Object Reference") (OtherComp :type "PrimitiveComponent Object Reference") (OtherBodyIndex :type Integer))
  (bind `_as丧尸_bp` (cast `/Game/创世之争/野怪/丧尸/丧尸_BP` OtherActor))
  (`KismetArrayLibrary.Array_RemoveItem` (`self.As AI BP`) `_as丧尸_bp`))

(event `self.ReceiveTick`
  (params (DeltaSeconds :type "Float (single-precision)"))
  (bind _as_ai_bp (`self.As AI BP`))
  (bind _targetai (`self.TargetAI`))
  (bind _output (`|GetArrayItem` _as_ai_bp))
  (`/Engine/EditorBlueprintResources/StandardMacros.IsValid` _targetai
    (:`Is Valid`
      (if (`/Game/创世之争/野怪/丧尸/丧尸_BP.Die` _targetai)
        (if (> (`KismetArrayLibrary.Array_Length` _as_ai_bp) 0) :!label _label
          (if (not (`/Game/创世之争/野怪/丧尸/丧尸_BP.Die` _output))
            (bind _output_get (set `self.TargetAI` _output))
            (`self.K2_AttachToActor` (`ChildActorComponent.ChildActor` (`self.激光Damage_BP`)) _output_get "None" "KeepRelative" "KeepRelative" "KeepWorld" true :!label _label_2)
            (`ActorComponent.SetActive` (`self.P_jiguangpaoLV2`) true true)
            (`/Game/创世之争/炮塔/激光/LV1/激光Damage_BP.ACFX_CS` (`self.FX`) true true)
            (`self.UpdateRotation_CS`))
          (else
            (`ActorComponent.SetActive` (`self.P_jiguangpaoLV2`) false true)
            (`/Game/创世之争/炮塔/激光/LV1/激光Damage_BP.ACFX_CS` (`self.FX`) false true)
            (`self.SetActorTickEnabled` false)))
        (else
          (goto _label_2))))
    (:`Is Not Valid`
      (goto _label))))

(event `UpdateRotation_CS`
  (bind (_returnvalue_roll _returnvalue_pitch _returnvalue_yaw) (`KismetMathLibrary.BreakRotator` (`self.K2_GetActorRotation`)))
  (`SceneComponent.K2_SetRelativeRotation` (`self.SM_激光炮LV1_攻击`) (`KismetMathLibrary.MakeRotator` 0.0 0.0 (+ (.yaw (`KismetMathLibrary.FindLookAtRotation` (`self.K2_GetActorLocation`) (`self.K2_GetActorLocation` (`self.TargetAI`)))) -90.0 (* _returnvalue_yaw -1.0))) false false)
  (`/Game/创世之争/炮塔/激光/LV1/激光Damage_BP.SetKill_CS` (`self.FX`) (`self.Kill`)))

(fn `UserConstructionScript`
  (bind _output_get (set `self.AllFX` (`|MakeArray` (`self.P_jiguangpaoLV2`))))
  (for _array_element _output_get
    (bind _asparticle_system_component (cast `ParticleSystemComponent` _array_element))
    (bind _aschild_actor_component (cast `ChildActorComponent` (`SceneComponent.GetChildComponent` _array_element 0)))
    (`FXSystemComponent.SetActorParameter` _asparticle_system_component "Target" (`ChildActorComponent.ChildActor` _aschild_actor_component))))