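; Laser hit actor for turret C that sweeps along a spline and damages zombies, hidden from BeginPlay until Start_CS.
; Start_CS reveals it and plays a timeline that moves it along the spline by inverted alpha, then calls EndCS on its Spawn reference.
; When a 丧尸_BP enters the capsule, every overlapping actor receives 999 damage through an interface message.
; The delayed call after finishing sets hidden to false again, so the actor stays visible.
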(event `self.ReceiveBeginPlay`
  (`self.SetActorHiddenInGame` true))

(event `Start_CS`
  (bind _spawn (`self.Spawn`))
  (`self.SetActorHiddenInGame` false)
  (bind (_direction `_新建轨道_0`) (`Timeline|时间轴_0` :!via `PlayFromStart`)
    (:`Update`
      (`self.K2_SetActorTransform` (`/Game/创世之争/野怪/BP/ASpline_BP.GetWorldPoint_CF` (`self.Spline`) (- 1.0 `_新建轨道_0`))))
    (:`Finished`
      (`/Engine/EditorBlueprintResources/StandardMacros.IsValid` _spawn
        (:`Is Valid`
          (`/Game/创世之争/野怪/BP/SpawnAI_BP.End_CS` _spawn))
        (:`Is Not Valid`
          _))
      (`KismetSystemLibrary.Delay` 0.5)
      (`self.SetActorHiddenInGame` false))))

(event `self.Capsule.OnComponentBeginOverlap`
  (params (OverlappedComponent :type "PrimitiveComponent Object Reference") (OtherActor :type "Actor Object Reference") (OtherComp :type "PrimitiveComponent Object Reference") (OtherBodyIndex :type Integer) (bFromSweep :type Boolean) (SweepResult :type "HitResult Structure (by ref)"))
  (cast `/Game/创世之争/野怪/丧尸/丧尸_BP` OtherActor)
  (for _array_element (`PrimitiveComponent.GetOverlappingActors` (`self.Capsule`) "/Script/Engine.Actor")
    (message `/Game/创世之争/野怪/BP/CSAI_Interface.CSIF_AI_Damage` _array_element 999.0)))

(fn `UserConstructionScript`)