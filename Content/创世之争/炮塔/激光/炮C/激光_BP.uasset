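; Laser turret (炮C) that runs a timed startup sequence and then fires at its hit actor, 激光击中BP.
; After a short BeginPlay delay, chained timelines run the startup, activate the laser point effect and raise the 上下 value before attacking.
; The attack hides that effect and branches on Int to start 激光FX_BP, the hit actor, or the Hit particle plus hit actor.
; Hit takes the hit actor as its Target parameter.
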(event `self.ReceiveBeginPlay`
  (`|ExecutionSequence`
    (:`then_0`
      (`FXSystemComponent.SetActorParameter` (`self.Hit`) "Target" (`self.激光击中_BP`)))
    (:`then_1`
      (`KismetSystemLibrary.Delay` 0.3)
      (`self.Start_CS`))))

(event `Start_CS`
  (`Timeline|时间轴_1` :!via `PlayFromStart`
    (:`Finished`
      (`ActorComponent.SetActive` (`self.P_jiguangPoint`) true false)
      (bind (_direction `_新建轨道_0`) (`Timeline|时间轴_3` :!via `PlayFromStart`)
        (:`Update`
          (set `self.上下` (`KismetMathLibrary.Lerp` -25.0 0.0 `_新建轨道_0`)))
        (:`Finished`
          (`self.Attack_CS`)
          (set `self.Fire` true))))))

(event `Attack_CS`
  (`SceneComponent.SetVisibility` (`self.P_jiguangPoint`) false false)
  (switch `int` (`self.Int`)
    (:`0`
      (bind _outactors (`GameplayStatics.GetAllActorsOfClass` "/Game/创世之争/炮塔/激光/炮C/激光FX_BP.激光FX_BP_C"))
      (`/Game/创世之争/炮塔/激光/炮C/激光FX_BP.StartFX_CS` (`|GetArrayItem` _outactors)))
    (:`1`
      (`/Game/创世之争/炮塔/激光/炮C/激光击中_BP.Start_CS` (`self.激光击中_BP`) :!label _label))
    (:`2`
      (`ActorComponent.SetActive` (`self.Hit`) true true)
      (goto _label))))

(event `Destroy_CS`)

(fn `UserConstructionScript`
  (`FXSystemComponent.SetActorParameter` (`self.Hit`) "Target" (`self.激光击中_BP`)))