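; Laser turret effect actor that fires a staged beam effect and sends overlapping zombies (丧尸_BP) flying.
; StartFX_CS activates the first particle, whose End parameter is bound to Start, while a timeline moves the actor from Start to End.
; On finish it staggers the other particles, enables per-Tick launching through capsule and sphere overlaps, then calls EndCS on SpawnAI_BP.
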(event `StartFX_CS`
  (`ActorComponent.SetActive` (`self.1`) true false)
  (`TimelineComponent.SetPlayRate` (`self.时间轴_0`) (`self.Rate`))
  (bind (_direction `_新建轨道_0`) (`Timeline|时间轴_0` :!via `PlayFromStart`)
    (:`Update`
      (`self.K2_SetActorLocation` (`KismetMathLibrary.VLerp` (`self.K2_GetActorLocation` (`self.Start`)) (`self.K2_GetActorLocation` (`self.End`)) `_新建轨道_0`)))
    (:`Finished`
      (`KismetSystemLibrary.Delay` 0.3)
      (`ActorComponent.SetActive` (`self.2`) true false)
      (`KismetSystemLibrary.Delay` 1.0)
      (`ActorComponent.SetActive` (`self.3`) true false)
      (set `self.01` true)
      (set `self.0` true)
      (`KismetSystemLibrary.Delay` 0.0)
      (`ActorComponent.SetActive` (`self.2`) false false)
      (`ActorComponent.SetActive` (`self.1`) false false)
      (`KismetSystemLibrary.Delay` 0.5)
      (bind _outactors (`GameplayStatics.GetAllActorsOfClass` "/Game/创世之争/野怪/BP/SpawnAI_BP.SpawnAI_BP_C"))
      (bind _output (`|GetArrayItem` _outactors))
      (`/Engine/EditorBlueprintResources/StandardMacros.IsValid` _output
        (:`Is Valid`
          (`/Game/创世之争/野怪/BP/SpawnAI_BP.End_CS` _output))))))

(event `self.ReceiveBeginPlay`
  (`FXSystemComponent.SetActorParameter` (`self.1`) "End" (`self.Start`))
  (set `self.SphereAll` (`|MakeArray` (`self.Sphere`) (`self.Sphere1`) (`self.Sphere2`) (`self.Sphere3`))))

(event `self.ReceiveTick`
  (params (DeltaSeconds :type "Float (single-precision)"))
  (bind _returnvalue (`self.K2_GetActorLocation`))
  (bind (_returnvalue_x _returnvalue_y _returnvalue_z) (`KismetMathLibrary.BreakVector` (- (`SceneComponent.K2_GetComponentLocation` (`self.Capsule`)) _returnvalue)))
  (`|ExecutionSequence`
    (:`then_0`
      (if (`self.0`)
        (for _array_element (`PrimitiveComponent.GetOverlappingActors` (`self.Capsule`) "/Script/Engine.Actor")
          (bind `_as丧尸_bp` (cast `/Game/创世之争/野怪/丧尸/丧尸_BP` _array_element))
          (message `/Game/创世之争/野怪/BP/CSAI_Interface.CSIF_AI_Fly` `_as丧尸_bp` (+ _returnvalue (`KismetMathLibrary.MakeVector` _returnvalue_x 0.0 _returnvalue_z)) (300.0 300.0 300.0)))))
    (:`then_1`
      (if (`self.01`)
        (for _array_element_2 (`self.SphereAll`)
          (for _array_element_3 (`PrimitiveComponent.GetOverlappingActors` _array_element_2 "/Script/Engine.Actor")
            (bind `_as丧尸_bp_2` (cast `/Game/创世之争/野怪/丧尸/丧尸_BP` _array_element_3))
            (message `/Game/创世之争/野怪/BP/CSAI_Interface.CSIF_AI_Fly` `_as丧尸_bp_2` (- (`SceneComponent.K2_GetComponentLocation` _array_element_2) (0.0 0.0 -150.0)) (300.0 300.0 300.0))))))))

(fn `UserConstructionScript`
  (`FXSystemComponent.SetActorParameter` (`self.1`) "End" (`self.Start`)))