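; Rocket artillery turret (火箭炮) that scales in on BeginPlay and activates once when a zombie (丧尸_BP) first overlaps its Box.
; Activation starts a looping firing animation with timeline-driven yaw sweep and a repeating timer that spawns rockets from two arrows.
; A delayed Stop flag changes the Kill value passed to later rockets.
; Overlapping zombies are tracked in an array, but look-at aiming is unconnected, so rotation ignores Target.
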(event `self.ReceiveTick`
  (params (DeltaSeconds :type "Float (single-precision)"))
  (`/Engine/EditorBlueprintResources/StandardMacros.IsValid` (`self.Target`)))

(event `StartFireCS`
  (bind _returnvalue (`KismetSystemLibrary.K2_SetTimerDelegate` (delegate `SPAWN_CS`) 0.5 true))
  (set `self.Timer` _returnvalue)
  (`KismetSystemLibrary.K2_PauseTimerHandle` (struct)))

(event `SPAWN_CS`
  (bind (_returnvalue_location _returnvalue_rotation _returnvalue_scale) (`KismetMathLibrary.BreakTransform` (`SceneComponent.K2_GetComponentToWorld` (`self.Arrow`))))
  (bind _returnvalue (not (`self.Stop`)))
  (`|SpawnActorFromClass` "/Game/创世之争/炮塔/火炮/火箭_BP_2.火箭_BP_2_C" (`KismetMathLibrary.MakeTransform` _returnvalue_location _returnvalue_rotation _returnvalue_scale) "AlwaysSpawn" "OverrideRootScale" null null _returnvalue null)
  (`|SpawnActorFromClass` "/Game/创世之争/炮塔/火炮/火箭_BP_2.火箭_BP_2_C" (`SceneComponent.K2_GetComponentToWorld` (`self.Arrow1`)) "AlwaysSpawn" "OverrideRootScale" null null _returnvalue null))

(event `self.ReceiveBeginPlay`
  (`|ExecutionSequence`
    (:`then_0`
      (set `self.AIIFX` (`|MakeArray` (`self.P_导弹_机枪3`) (`self.P_导弹_机枪4`) (`self.P_导弹_机枪5`) (`self.P_导弹_机枪6`) (`self.P_导弹_机枪1`) (`self.P_导弹_机枪2`)))
      (`KismetSystemLibrary.Delay` 0.5))
    (:`then_1`
      (bind (_direction `_新建轨道_0`) (`Timeline|时间轴_2` :!via `PlayFromStart`)
        (:`Update`
          (bind _output_get (set `self.大小` `_新建轨道_0`))
          (`SceneComponent.SetRelativeScale3D` (`self.04炮台`) (`KismetMathLibrary.Conv_DoubleToVector` _output_get))
          (`SceneComponent.SetRelativeScale3D` (`self.04炮身`) (* (0.6 0.6 1.0) _output_get)))))))

(event `self.CSIF_Start`
  (`self.Rotation_CS`)
  (`self.StartFireCS`))

(event `Rotation_CS`
  (`SkeletalMeshComponent.PlayAnimation` (`self.04炮台`) "/Game/创世之争/炮塔/火炮/pao5/04炮台_开枪_2.04炮台_开枪_2" true)
  (`TimelineComponent.SetPlayRate` (`self.时间轴_3`) (`self.Rate`))
  (bind (_direction `_新建轨道_0`) (`Timeline|时间轴_3` :!via `PlayFromStart`)
    (:`Update`
      (`SceneComponent.K2_SetRelativeRotation` (`self.04炮台`) (`KismetMathLibrary.MakeRotator` 0.0 0.0 (* `_新建轨道_0` (`self.RangeYaw`))) false false))))

(event `Start_CS`
  (bind (_direction `_新建轨道_0`) (`Timeline|时间轴_0` :!via `PlayFromStart`)
    (:`Update`
      (`SceneComponent.SetRelativeScale3D` (`self.04炮身`) (* (0.6 0.6 1.0) `_新建轨道_0`))
      (`SceneComponent.SetRelativeScale3D` (`self.04炮台`) (`KismetMathLibrary.Conv_DoubleToVector` (* `_新建轨道_0` 1.0))))
    (:`Finished`
      (`self.Rotation_CS`))))

(event `ActiveFX_CS`
  (`ActorComponent.SetActive` (`self.AIIFX`) true false))

(event `self.Box.OnComponentBeginOverlap`
  (params (OverlappedComponent :type "PrimitiveComponent Object Reference") (OtherActor :type "Actor Object Reference") (OtherComp :type "PrimitiveComponent Object Reference") (OtherBodyIndex :type Integer) (bFromSweep :type Boolean) (SweepResult :type "HitResult Structure (by ref)"))
  (bind `_as丧尸_bp` (cast `/Game/创世之争/野怪/丧尸/丧尸_BP` OtherActor))
  (`KismetArrayLibrary.Array_Add` (`self.As AI BP`) `_as丧尸_bp`)
  (`/Engine/EditorBlueprintResources/StandardMacros.IsValid` (`self.Target`)
    (:`Is Valid`
      _)
    (:`Is Not Valid`
      (set `self.Target` null)))
  (`/Engine/EditorBlueprintResources/StandardMacros.DoOnce` false
    (:`Completed`
      (`self.CSIF_Start`)
      (`KismetSystemLibrary.Delay` 4.0)
      (set `self.Stop` true))))

(event `self.Box.OnComponentEndOverlap`
  (params (OverlappedComponent :type "PrimitiveComponent Object Reference") (OtherActor :type "Actor Object Reference") (OtherComp :type "PrimitiveComponent Object Reference") (OtherBodyIndex :type Integer))
  (bind _output (`|GetArrayItem` (`self.As AI BP`)))
  (bind `_as丧尸_bp` (cast `/Game/创世之争/野怪/丧尸/丧尸_BP` OtherActor))
  (`KismetArrayLibrary.Array_RemoveItem` (`self.As AI BP`) `_as丧尸_bp`)
  (if (== `_as丧尸_bp` (`self.Target`))
    (`/Engine/EditorBlueprintResources/StandardMacros.IsValid` _output
      (:`Is Valid`
        (set `self.Target` _output)))))

(fn `CSIF_AI_State`
  (returns (Die :type Boolean) (Speed :type "Float (double-precision)"))
  (return false 0.0))

(fn `UserConstructionScript`)