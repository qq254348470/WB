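; Soldier unit character (兵种) with team-colored, camera-facing health bar, firing randomly scattered 箭_BP arrows at its target or ahead.
; BeginPlay picks display or random-point movement; AI move orders go through 兵种_Contro, while spline movement is stubbed.
; Interface calls apply damage, launch non-boss units into ragdoll death, and expose attack, velocity and aim for animation.
; Timelines fade a dynamic material, then flag the unit 敌方 (enemy).
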(event `UpdateM_CS`
  (bind _dy_m (`self.Dy_M`))
  ;[1 1 1] 出现变化
  (`/Engine/EditorBlueprintResources/StandardMacros.IsValid` _dy_m
    (:`Is Valid`
      (set `self.Attack` false)
      (`PrimitiveComponent.SetMaterial` (`self.Mesh`) 0 _dy_m)
      (`ActorComponent.SetActive` (`self.P_paotashengji`) true true)
      (bind (_direction `_新建轨道_0`) (`Timeline|时间轴_2` :!via `PlayFromStart`)
        (:`Update`
          (`MaterialInstanceDynamic.SetScalarParameterValue` (`self.Dy_M`) "Alpha" `_新建轨道_0`))
        (:`Finished`
          (set `self.敌方` true))))))

(event `self.ReceiveBeginPlay`
  (`|ExecutionSequence`
    (:`then_0`
      (`self.InitInfo_CS`))
    (:`then_1`
      (switch `/Game/创世之争/兵种/BP/AI/Enum/Enum_移动类型` (`self.Enum_移动类型`)
        (:`NewEnumerator0`
          (`self.Show Anim CF` (`self.Enum_兵种状态(展示)`)))
        (:`NewEnumerator7`
          (`self.SplineMove_CS`))
        (:`NewEnumerator5`
          (set `self.Random` false))
        (:`NewEnumerator1`
          (set `self.Random` true))))
    (:`then_2`
      (add `self.ResetMoveEventDis` (delegate `MoveEnd`)))))

(event `InRange_CS`
  (bind _dy_m (`self.Dy_M`))
  ;[1 1 1] 材质变化
  (`/Engine/EditorBlueprintResources/StandardMacros.IsValid` _dy_m
    (:`Is Valid`
      (`/Engine/EditorBlueprintResources/StandardMacros.DoOnce` false
        (:`Completed`
          (set `self.Attack` false)
          (`PrimitiveComponent.SetMaterial` (`self.Mesh`) 0 _dy_m)
          (`ActorComponent.SetActive` (`self.P_paotashengji`) true true)
          (`SceneComponent.SetVisibility` (`self.Plane`) true false)
          (bind (_direction `_新建轨道_0`) (`Timeline|时间轴_0` :!via `PlayFromStart`)
            (:`Update`
              (`MaterialInstanceDynamic.SetScalarParameterValue` (`self.Dy_M`) "Alpha" `_新建轨道_0`))
            (:`Finished`
              (set `self.敌方` true))))))))

(event `MoveEnd`
  (if (not (`self.End`))
    (set `self.Attack` true)
    (`NavMovementComponent.StopActiveMovement` (`self.CharacterMovement`))))

(event `InitInfo_CS`
  (bind _returnvalue (`self.K2_GetActorLocation`))
  (bind _dy_m (`self.Dy_M`))
  (`|ExecutionSequence`
    (:`then_0`
      ;[1 1 1] 血条颜色设置
      (bind _ashp_umg (cast `/Game/创世之争/兵种/BP/AI/兵种HP_UMG` (`WidgetComponent.GetUserWidgetObject` (`self.Widget`))))
      (bind _output_get (set `self.HP UMG` _ashp_umg))
      (`/Game/创世之争/兵种/BP/AI/兵种HP_UMG.ChangeColor_CF` _output_get (select `/Game/创世之争/兵种/BP/AI/Enum/Enum_阵营` "NewEnumerator0" :`NewEnumerator5` (struct :`R` 1.0 :`A` 1.0) :`NewEnumerator1` (struct :`B` 1.0 :`A` 1.0) :`NewEnumerator3` (struct :`G` 1.0 :`A` 1.0) :!type "LinearColor Structure"))
      (bind _output_get_2 (set `self.Max_HP` 100.0))
      (set `self.Current_HP` _output_get_2))
    (:`then_1`
      ;[1 1 1] 初始位置设置
      (set `self.StartPoint` (`self.GetTransform`))
      (set `self.NewPoint` _returnvalue)
      (`/Engine/EditorBlueprintResources/StandardMacros.IsValid` null
        (:`Is Valid`
          (set `self.Offset` (- _returnvalue (`self.K2_GetActorLocation`))))))
    (:`then_2`
      (if (`self.敌方`)
        (`/Engine/EditorBlueprintResources/StandardMacros.IsValid` _dy_m
          (:`Is Valid`
            (`PrimitiveComponent.SetMaterial` (`self.Mesh`) 0 _dy_m)))))))

(event `SplineMove_CS`
  ;[1 1 1] 沿样条线移动
  (`/Engine/EditorBlueprintResources/StandardMacros.IsValid` null))

(event `ChangeRate_CS`
  (params (Reset :type Boolean))
  (bind `_时间轴_样条线` (`self.时间轴_样条线`))
  ;[1 1 1] 改变速度
  (if Reset
    (`TimelineComponent.SetPlayRate` `_时间轴_样条线` (`self.样条线移动速率`))
    (else
      (bind (_direction _rate) (`Timeline|时间轴_1` :!via `PlayFromStart`)
        (:`Update`
          (`TimelineComponent.SetPlayRate` `_时间轴_样条线` _rate))))))

(event `/Game/创世之争/兵种/BP/CSIF_AI.CSIF_MakeDamage`
  (params (Damage :type "Float (single-precision)"))
  ;[1 1 1] 伤害判定，死亡，销毁
  (bind _die (`self.Damage_CF` Damage))
  (if _die
    (`|ExecutionSequence`
      (:`then_0`
        (set `self.展示` false)
        (`TimelineComponent.Stop` (`self.时间轴_样条线`))
        (`NavMovementComponent.StopActiveMovement` (`self.CharacterMovement`))
        (`self.SetActorEnableCollision` false))
      (:`then_1`
        (set `self.Die` true)
        (`KismetSystemLibrary.Delay` (`KismetMathLibrary.RandomFloatInRange` 2.0 4.0))
        (`self.K2_DestroyActor`)))))

(event `self.ReceiveTick`
  (params (DeltaSeconds :type "Float (single-precision)"))
  ;[1 1 1] 血条朝向，攻击手目标朝向
  (`KismetSystemLibrary.Delay` 0.1)
  (`self.UpdateHPRotation_CF`))

(event `/Game/创世之争/兵种/BP/CSIF_AI.CSIF_Fly`
  (params (Point :type "Vector Structure") (Speed :type "Vector Structure"))
  (bind _mesh (`self.Mesh`))
  (bind (_returnvalue_x _returnvalue_y) (`KismetMathLibrary.BreakVector` (* (`KismetMathLibrary.Normal` (- (`self.K2_GetActorLocation`) Point)) Speed)))
  ;[1 1 1] 击飞
  (if (`self.Boss`)
    _
    (elif (not (`self.Die`))
      (set `self.Die` true)
      (`TimelineComponent.Stop` (`self.时间轴_样条线`))
      (`MovementComponent.StopMovementImmediately` (`self.CharacterMovement`))
      (`self.LaunchCharacter` (`KismetMathLibrary.MakeVector` _returnvalue_x _returnvalue_y (.z Speed)) true true) ; 1000
      (`KismetSystemLibrary.Delay` 0.3)
      (`SkeletalMeshComponent.SetAllBodiesSimulatePhysics` _mesh true)
      (`SkeletalMeshComponent.SetAllBodiesPhysicsBlendWeight` _mesh 1.0 true)
      (`PrimitiveComponent.SetCollisionEnabled` _mesh "QueryAndPhysics")
      (`PrimitiveComponent.SetCollisionEnabled` (`self.CapsuleComponent`) "NoCollision")
      (`KismetSystemLibrary.Delay` (`KismetMathLibrary.RandomFloatInRange` 1.0 3.0))
      (`self.K2_DestroyActor`))))

(event `/Game/创世之争/兵种/BP/CSIF_AI.CSIF_Attack`
  (bind _aimtarget (`self.AimTarget`))
  (bind _location (.location (`SceneComponent.K2_GetComponentToWorld` (`self.Arrow1`))))
  (bind _location_2 (.location (`SceneComponent.K2_GetComponentToWorld` (`self.Arrow1`))))
  (bind _location_3 (.location (`SceneComponent.K2_GetComponentToWorld` (`self.Arrow1`))))
  (bind _returnvalue (`KismetMathLibrary.RandomPointInBoundingBox` (+ (`self.K2_GetActorLocation` (`self.目标`)) (`KismetMathLibrary.MakeVector` 0.0 0.0 (/ (`CapsuleComponent.CapsuleHalfHeight` (`self.CapsuleComponent`)) -1.0))) (`self.AimBox Extent`)))
  (bind _returnvalue_2 (`KismetMathLibrary.RandomPointInBoundingBox` (+ (`self.K2_GetActorLocation` _aimtarget) (`KismetMathLibrary.MakeVector` 0.0 0.0 (/ (`CapsuleComponent.CapsuleHalfHeight` (`self.CapsuleComponent`)) -1.0))) (`self.AimBox Extent`)))
  (bind _returnvalue_3 (+ (+ (`self.K2_GetActorLocation` self) (+ (* (`self.GetActorUpVector` self) 250.0) (* (`self.GetActorForwardVector` self) 1350.0))) (`KismetMathLibrary.MakeVector` 0.0 0.0 (/ (`CapsuleComponent.CapsuleHalfHeight` (`self.CapsuleComponent`)) 0.0))))
  ;[1 0 0] 攻击
  (`|ExecutionSequence`
    (:`then_1`
      (`/Engine/EditorBlueprintResources/StandardMacros.IsValid` (`self.目标`)
        (:`Is Valid`
          (for _ (range 2)
            (set `self.AimBox Extent` (300.0 300.0 100.0))
            (`|SpawnActorFromClass` "/Game/创世之争/兵种/BP/箭_BP.箭_BP_C" (`KismetMathLibrary.MakeTransform` _location (struct) (.scale (`SceneComponent.K2_GetComponentToWorld` (`self.Arrow1`)))) "Undefined" "OverrideRootScale" null _location -0.0 _returnvalue (`KismetMathLibrary.MapRangeClamped` (`KismetMathLibrary.VSize` (- (`self.K2_GetActorLocation` self) _returnvalue)) 500.0 2000.0 0.5 1.0) (`self.Enum_阵营`) self) ; 111--980\n0.3--0
          ))
        (:`Is Not Valid`
          (`/Engine/EditorBlueprintResources/StandardMacros.IsValid` _aimtarget
            (:`Is Valid`
              (for _ (range 1)
                (set `self.AimBox Extent` (70.0 70.0 0.0))
                (`|SpawnActorFromClass` "/Game/创世之争/兵种/BP/箭_BP.箭_BP_C" (`KismetMathLibrary.MakeTransform` _location_2 (struct) (.scale (`SceneComponent.K2_GetComponentToWorld` (`self.Arrow1`)))) "Undefined" "OverrideRootScale" null _location_2 -980.0 _returnvalue_2 (`KismetMathLibrary.MapRangeClamped` (`KismetMathLibrary.VSize` (- (`self.K2_GetActorLocation` self) _returnvalue_2)) 0.0 800.0 0.1 0.5) (`self.Enum_阵营`) self) ; 111--980\n0.3--0
              ))
            (:`Is Not Valid`
              (for _ (range 3)
                (bind _output_get (set `self.Arrow_Point` (`KismetMathLibrary.RandomPointInBoundingBox` _returnvalue_3 (100.0 100.0 100.0))))
                (bind _returnvalue_4 (`|SpawnActorFromClass` "/Game/创世之争/兵种/BP/箭_BP.箭_BP_C" (`KismetMathLibrary.MakeTransform` _location_3 (struct) (* (.scale (`SceneComponent.K2_GetComponentToWorld` (`self.Arrow1`))) 2.0)) "Undefined" "OverrideRootScale" null _location_3 -1980.0 _output_get (`KismetMathLibrary.MapRangeClamped` (`KismetMathLibrary.VSize` (- _returnvalue_3 (`self.K2_GetActorLocation` self))) 0.0 800.0 0.1 0.5) (`self.Enum_阵营`) self)) ; 111--980\n0.3--0
                (`/Game/创世之争/兵种/BP/箭_BP.Die_CS` _returnvalue_4)))))))))

(event `UpdatePoint_CS`
  (bind _aimovetotarget (`self.AimovetoTarget`))
  (`|ExecutionSequence`
    (:`then_0`
      (`/Engine/EditorBlueprintResources/StandardMacros.DoOnce` false
        (:`Completed`
          ;[1 1 1] AI
          (set `self.Attack` false))))
    (:`then_1`
      (`ActorComponent.SetActive` (`self.CharacterMovement`) true true)
      (if (`self.Random`)
        (bind _output_get (set `self.NewPoint` (`NavigationSystemV1.K2_GetRandomReachablePointInRadius` (`NavigationSystemV1.GetNavigationSystem`) (`self.NewPoint`) 500.0 null "/Game/创世之争/兵种/BP/AI/CS_NavFilter.CS_NavFilter_C")))
        (`KismetSystemLibrary.DrawDebugSphere` _output_get 15.0 12 (struct :`R` 1.0 :`A` 1.0) 1.0 3.0)
        (`/Engine/EditorBlueprintResources/StandardMacros.DoOnce` false
          (:`Completed`
            (set `CharacterMovementComponent.MaxWalkSpeed` 400.0 (`self.CharacterMovement`))))
        (else
          (`/Engine/EditorBlueprintResources/StandardMacros.IsValid` _aimovetotarget
            (:`Is Valid`
              (set `self.NewPoint` (`self.K2_GetActorLocation` _aimovetotarget)))
            (:`Is Not Valid`
              (set `self.NewPoint` (`self.UpdatePoint`)))))))))

(event `Run_CS`
  (bind _startpoint_location (`KismetMathLibrary.BreakTransform` (`self.StartPoint`)))
  (bind _returnvalue (+ (* (`KismetMathLibrary.Normal` (- (`self.K2_GetActorLocation` (`self.目标`)) _startpoint_location)) -1500.0) _startpoint_location))
  ;[1 1 1] 反方向逃离目标
  (`KismetSystemLibrary.DrawDebugArrow` _returnvalue (`NavigationSystemV1.K2_GetRandomReachablePointInRadius` _returnvalue 250.0 null null) 10.0 (struct :`R` 1.0 :`A` 1.0) 10.0 10.0)
  (`|AIMoveTo` self (`KismetMathLibrary.RandomPointInBoundingBox` _returnvalue (250.0 250.0 0.0)) null 50.0))

(event `CheckPoint_CS`
  (bind (_returnvalue_x _returnvalue_y) (`KismetMathLibrary.BreakVector` (`self.K2_GetActorLocation`)))
  (bind (_newpoint_x _newpoint_y) (`KismetMathLibrary.BreakVector` (`self.NewPoint`)))
  ;[1 1 1] AI
  (if (<= (`KismetMathLibrary.VSize` (- (`KismetMathLibrary.MakeVector` _returnvalue_x _returnvalue_y) (`KismetMathLibrary.MakeVector` _newpoint_x _newpoint_y))) 50.0)
    (`self.UpdatePoint_CS`)
    (goto _label :!via `Reset`)
    (else
      (`/Engine/EditorBlueprintResources/StandardMacros.DoOnce` false :!label _label
        (:`Completed`
          (`/Engine/EditorBlueprintResources/StandardMacros.IsValid` (`self.目标`)
            (:`Is Not Valid`
              (set `CharacterMovementComponent.MaxWalkSpeed` (`self.Max Walk Speed`) (`self.CharacterMovement`)))))))))

(event `AImoveToTarget_BP`
  (params (Destination :type Integer) (UpdatePoint :type "Vector Structure") (TargetActor :type "Actor Object Reference"))
  (bind _returnvalue (`self.K2_GetActorLocation` TargetActor))
  (switch `int` Destination
    (:`0`
      (set `self.AITarget` TargetActor)
      (bind `_as兵种_contro` (cast `/Game/创世之争/兵种/BP/AI/兵种_Contro` (`AIBlueprintHelperLibrary.GetAIController` self)))
      (`/Game/创世之争/兵种/BP/AI/兵种_Contro.UpdateState_CS` `_as兵种_contro` UpdatePoint TargetActor)
      (`self.ActiveFX_CS`))
    (:`1`
      (`KismetSystemLibrary.DrawDebugPoint` _returnvalue 50.0 (struct :`R` 1.0 :`A` 1.0) 10.0)
      (`|AIMoveTo` self _returnvalue null 50.0 true))))

(event `ActiveFX_CS`)

(event `self.ReceiveEndPlay`
  (params (EndPlayReason :type "EEndPlayReason Enum" :default "Destroyed"))
  (`self.DestroyDis` self))

(event `Attach_CS`
  (params (`目标` :type "Actor Object Reference"))
  ;[1 1 1] 附加，本意用于被箭射中后绑定在骨骼上，一起运动
  (`self.K2_AttachToComponent` `目标` (`self.Mesh`) "None" "KeepWorld" "KeepWorld" "KeepWorld" true))

(fn `CSIF_AniInfo`
  (returns (Attack :type Boolean) (Velocity :type "Vector Structure") (Die :type Boolean) (Rotation :type "Rotator Structure"))
  (return (`self.Attack`) (`MovementComponent.Velocity` (`self.CharacterMovement`)) (`self.Die`) (`self.AimRotation`)))

(fn `CSIF_Get阵营`
  (returns (AI :type "/Game/创世之争/兵种/BP/AI/Enum/Enum_阵营 Enum"))
  (return (`self.Enum_阵营`)))

(fn `Damage_CF`
  (params (Damage :type "Float (double-precision)"))
  (returns (Die :type Boolean))
  (bind _output_get (set `self.Current_HP` (- (`self.Current_HP`) Damage)))
  (`/Game/创世之争/兵种/BP/AI/兵种HP_UMG.UpdateHP_CS` (`self.HP UMG`) (/ _output_get (`self.Max_HP`)))
  (return (<= _output_get 0.01)))

(fn `Init Info CF`
  (params (`Enum_阵营` :type "/Game/创世之争/兵种/BP/AI/Enum/Enum_阵营 Enum" :default "NewEnumerator0") (`Enum_兵种状态(展示)` :type "/Game/创世之争/兵种/BP/AI/Enum/Enum_兵种状态 Enum" :default "NewEnumerator6") (Value :type "Integer (by ref)") (Parent :type "MaterialInterface Object Reference"))
  (set `self.Enum_阵营` `Enum_阵营`)
  (set `self.Enum_兵种状态(展示)` `Enum_兵种状态(展示)`)
  (bind _output_get (set `self.Index` Value))
  (`TextRenderComponent.K2_SetText` (`self.TextRender`) (`KismetTextLibrary.Conv_IntToText` _output_get))
  (if (!= Parent null)
    (set `self.Parent` Parent)))

(fn `LockRotation_CF`
  (bind (_returnvalue_roll _returnvalue_pitch _returnvalue_yaw) (`KismetMathLibrary.BreakRotator` (`self.K2_GetActorRotation`)))
  (bind _returnvalue (`self.K2_GetActorLocation` (`self.目标`)))
  (bind _returnvalue_2 (`KismetMathLibrary.FindLookAtRotation` (`self.K2_GetActorLocation` self) (`KismetMathLibrary.RandomPointInBoundingBox` _returnvalue (`self.AimBox Extent`))))
  (`/Engine/EditorBlueprintResources/StandardMacros.IsValid` (`self.目标`)
    (:`Is Valid`
      (if (not (== _returnvalue (`self.AimPoint`) :`ErrorTolerance` 1.0))
        (set `self.AimPoint` _returnvalue)
        (`self.K2_SetActorRotation` (`KismetMathLibrary.MakeRotator` 0.0 0.0 (.yaw _returnvalue_2)))
        (set `self.AimRotation` (`KismetMathLibrary.MakeRotator` (- (- _returnvalue_pitch (.pitch _returnvalue_2)) (`self.PitchOffset`)) (- (.roll _returnvalue_2) _returnvalue_roll) (- (- (.yaw _returnvalue_2) _returnvalue_yaw) (`self.YawOffset`))))))))

(fn `Show Anim CF`
  (params (Selection :type "/Game/创世之争/兵种/BP/AI/Enum/Enum_兵种状态 Enum" :default "NewEnumerator6"))
  (set `self.展示` false)
  (set `self.Attack` false)
  (switch `/Game/创世之争/兵种/BP/AI/Enum/Enum_兵种状态` Selection
    (:`NewEnumerator7`
      (set `self.展示` true))
    (:`NewEnumerator5`
      (set `self.Attack` true))))

(fn `UpdateHPRotation_CF`
  (bind _widget (`self.Widget`))
  (bind (_returnvalue_x _returnvalue_y _returnvalue_z) (`KismetMathLibrary.BreakVector` (`self.K2_GetActorLocation` (`GameplayStatics.GetPlayerCameraManager` 0))))
  (bind (_returnvalue_roll _returnvalue_pitch _returnvalue_yaw) (`KismetMathLibrary.BreakRotator` (`KismetMathLibrary.FindLookAtRotation` (`SceneComponent.K2_GetComponentLocation` _widget) (`KismetMathLibrary.MakeVector` _returnvalue_x _returnvalue_y _returnvalue_z))))
  (`/Engine/EditorBlueprintResources/StandardMacros.IsValid` _widget
    (:`Is Valid`
      (`SceneComponent.K2_SetWorldRotation` _widget (`KismetMathLibrary.MakeRotator` 0.0 _returnvalue_pitch _returnvalue_yaw) false false))))

(fn `UserConstructionScript`
  (bind _returnvalue (`KismetMaterialLibrary.CreateDynamicMaterialInstance` (`self.Parent`)))
  (set `self.Dy_M` _returnvalue))