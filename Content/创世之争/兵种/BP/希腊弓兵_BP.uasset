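; Greek archer troop Blueprint (希腊弓兵), whose only working logic is a knock-away death.
; CSIFFly runs once for non-boss units, setting Die, stopping the spline timeline and movement, then launching the character away from the given point.
; It then disables capsule collision and destroys the actor after a short random delay.
; Overlap and MoveEnd events are empty; ragdoll and AI-move nodes are left unconnected.
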(event `self.Box.OnComponentBeginOverlap`
  (params (OverlappedComponent :type "PrimitiveComponent Object Reference") (OtherActor :type "Actor Object Reference") (OtherComp :type "PrimitiveComponent Object Reference") (OtherBodyIndex :type Integer) (bFromSweep :type Boolean) (SweepResult :type "HitResult Structure (by ref)")))

(event `self.MoveEnd`)

(event `/Game/创世之争/兵种/BP/CSIF_AI.CSIF_Fly`
  (params (Point :type "Vector Structure") (Speed :type "Vector Structure"))
  (bind (_returnvalue_x _returnvalue_y) (`KismetMathLibrary.BreakVector` (* (`KismetMathLibrary.Normal` (- (`self.K2_GetActorLocation`) Point)) Speed)))
  (if (`self.Boss`)
    _
    (elif (not (`self.Die`))
      (set `self.Die` true)
      (`TimelineComponent.Stop` (`self.时间轴_样条线`))
      (`MovementComponent.StopMovementImmediately` (`self.CharacterMovement`))
      (`self.LaunchCharacter` (`KismetMathLibrary.MakeVector` _returnvalue_x _returnvalue_y (.z Speed)) true true) ; 1000
      (`KismetSystemLibrary.Delay` 0.3)
      (`PrimitiveComponent.SetCollisionEnabled` (`self.CapsuleComponent`) "NoCollision")
      (`KismetSystemLibrary.Delay` (`KismetMathLibrary.RandomFloatInRange` 1.0 3.0))
      (`self.K2_DestroyActor`))))

(fn `UserConstructionScript`
  (`parent.UserConstructionScript`))