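; Greek cavalry unit Blueprint (希腊骑1兵) for 创世之争, extending a parent class with effect and state events.
; CustomEvent runs once, clearing Attack, applying dynamic material DyM, firing a particle effect and animating Alpha by timeline before setting 敌方 (enemy) true.
; CSIFAttack activates the charge particle.
; ActiveFXCS uses a MultiGate whose Out 1 plays that particle, then destroys the actor after a delay.
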(event `self.ReceiveTick`
  (params (DeltaSeconds :type "Float (single-precision)"))
  (`parent.ReceiveTick` DeltaSeconds))

(event `CustomEvent`
  (bind _dy_m (`self.Dy_M`))
  (`/Engine/EditorBlueprintResources/StandardMacros.IsValid` _dy_m
    (:`Is Valid`
      (`/Engine/EditorBlueprintResources/StandardMacros.DoOnce` false
        (:`Completed`
          (set `self.Attack` false)
          (`PrimitiveComponent.SetMaterial` (`self.Mesh`) 0 _dy_m)
          (`ActorComponent.SetActive` (`self.P_paotashengji`) true true)
          (bind (_direction `_新建轨道_0`) (`Timeline|时间轴_3` :!via `PlayFromStart`)
            (:`Update`
              (`MaterialInstanceDynamic.SetScalarParameterValue` (`self.Dy_M`) "Alpha" `_新建轨道_0`))
            (:`Finished`
              (set `self.敌方` true))))))))

(event `/Game/创世之争/兵种/BP/CSIF_AI.CSIF_Attack`
  (`ActorComponent.SetActive` (`self.P_冲刺_H`) true true))

(event `self.MoveEnd`)

(event `self.ActiveFX_CS`
  (`|MultiGate` false false 0
    (:`Out 1`
      (`ActorComponent.SetActive` (`self.P_冲刺_H`) true true)
      (`KismetSystemLibrary.Delay` 1.3)
      (`ActorComponent.SetActive` (`self.P_冲刺_H`) false true)
      (`KismetSystemLibrary.Delay` 0.0)
      (`self.K2_DestroyActor`))))

(event `self.Box.OnComponentBeginOverlap`
  (params (OverlappedComponent :type "PrimitiveComponent Object Reference") (OtherActor :type "Actor Object Reference") (OtherComp :type "PrimitiveComponent Object Reference") (OtherBodyIndex :type Integer) (bFromSweep :type Boolean) (SweepResult :type "HitResult Structure (by ref)")))

(fn `UserConstructionScript`
  (`parent.UserConstructionScript`))