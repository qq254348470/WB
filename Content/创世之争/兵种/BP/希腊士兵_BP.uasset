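; Greek soldier unit Blueprint (希腊士兵), a child class that adds particle effects to attack and CS events.
; CSIFAttack restarts its particle system, while ActiveFXCS passes a non-looping MultiGate that turns on the blue light-shield effect (P光盾蓝) only at its third output.
; Stop_CS sets a condition flag, calls CSIFMakeDamage with a very large value and switches the shield off.
; Overlap and movement-end events are empty, and older box-collision logic is left disconnected.
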(event `self.CSIF_Attack`
  (`ActorComponent.SetActive` (`self.ParticleSystem`) true true))

(event `self.MoveEnd`)

(event `self.ActiveFX_CS`
  (`|MultiGate` false false 0
    (:`Out 2`
      (`ActorComponent.SetActive` (`self.P_光盾_蓝`) true true))))

(event `self.Box.OnComponentBeginOverlap`
  (params (OverlappedComponent :type "PrimitiveComponent Object Reference") (OtherActor :type "Actor Object Reference") (OtherComp :type "PrimitiveComponent Object Reference") (OtherBodyIndex :type Integer) (bFromSweep :type Boolean) (SweepResult :type "HitResult Structure (by ref)")))

(event `Stop_CS`
  (set `self.Condition` true)
  (`self.CSIF_MakeDamage` 999.0)
  (`ActorComponent.SetActive` (`self.P_光盾_蓝`) false true))

(event `ACFX_CS`
  (params (bNewActive :type Boolean)))

(fn `UserConstructionScript`
  (`parent.UserConstructionScript`))